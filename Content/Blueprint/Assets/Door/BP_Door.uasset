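; BP_Door is a door Blueprint that tells the player a puzzle is not yet solved.
; When BP_Vum enters its Box trigger, it stores the player and, if IsDoorOpened is false, shows a BP_PuzzleNotSolved widget.
; Leaving the trigger removes the stored widget without a validity check.
; The file holds no logic that opens or moves the door.
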(event OnComponentBeginOverlap(Box)
  (params (OverlappedComponent :type Primitive%20Component%20Object%20Reference) (OtherActor :type Actor%20Object%20Reference) (OtherComp :type Primitive%20Component%20Object%20Reference) (OtherBodyIndex :type Integer) (bFromSweep :type Boolean) (SweepResult :type Hit%20Result%20Structure%20%28by%20ref%29))
  (bind _asbp_vum (Utilities|Casting|CastToBP_Vum OtherActor))
  (Variables|Default|SetPlayer_Ref _asbp_vum)
  (if (not (Variables|/Game/Blueprint/Player_Vum/BP_Vum.BP_Vum_C|GetisDoorOpened? (Variables|Default|GetPlayer_Ref)))
    (bind _returnvalue (UserInterface|CreateWidget "/Game/Blueprint/Assets/Door/BP_PuzzleNotSolved.BP_PuzzleNotSolved_C"))
    (bind _output_get (Variables|Default|SetWidgetRef _returnvalue))
    (UserInterface|Viewport|AddtoViewport _output_get 0)))

(event OnComponentEndOverlap(Box)
  (params (OverlappedComponent :type Primitive%20Component%20Object%20Reference) (OtherActor :type Actor%20Object%20Reference) (OtherComp :type Primitive%20Component%20Object%20Reference) (OtherBodyIndex :type Integer))
  (Utilities|Casting|CastToBP_Vum OtherActor)
  (Widget|RemovefromParent (Variables|Default|GetWidgetRef)))

(event EventBeginPlay)

(event Collision|EventActorBeginOverlap
  (params (OtherActor :type Actor%20Object%20Reference)))

(event EventTick
  (params (DeltaSeconds :type Float%20%28single-precision%29)))

(fn ConstructionScript)