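; BP_GravityFloor is a floor actor that inverts gravity for BP_Vum while it overlaps the ButtonCollision component.
; On overlap begin it stores the character, applies a small downward force, sets a negative gravity scale and sets extremely high linear damping on the capsule.
; On overlap end it restores normal gravity and low damping through the stored reference.
; A node that would set the floor's pitch is left unconnected.
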(event OnComponentBeginOverlap(Buttoncollision)
  (params (OverlappedComponent :type Primitive%20Component%20Object%20Reference) (OtherActor :type Actor%20Object%20Reference) (OtherComp :type Primitive%20Component%20Object%20Reference) (OtherBodyIndex :type Integer) (bFromSweep :type Boolean) (SweepResult :type Hit%20Result%20Structure%20%28by%20ref%29))
  (bind _asbp_vum (Utilities|Casting|CastToBP_Vum OtherActor))
  (bind _output_get (Variables|Default|SetPlayerVum%20Ref _asbp_vum))
  (Physics|AddForce (Variables|/Script/Engine.Character|GetCharacterMovement _output_get) "0.000000,0.000000,-20.000000")
  (Variables|/Script/Engine.CharacterMovementComponent|SetGravityScale (Variables|/Script/Engine.Character|GetCharacterMovement _output_get) -1.0)
  (Class|PrimitiveComponent|SetLinearDamping (Variables|/Script/Engine.Character|GetCapsuleComponent _output_get) 1e+09))

(event OnComponentEndOverlap(Buttoncollision)
  (params (OverlappedComponent :type Primitive%20Component%20Object%20Reference) (OtherActor :type Actor%20Object%20Reference) (OtherComp :type Primitive%20Component%20Object%20Reference) (OtherBodyIndex :type Integer))
  (bind _playervum_ref (Variables|Default|GetPlayerVum%20Ref))
  (Utilities|Casting|CastToBP_Vum OtherActor)
  (Variables|/Script/Engine.CharacterMovementComponent|SetGravityScale (Variables|/Script/Engine.Character|GetCharacterMovement _playervum_ref) 1.0)
  (Class|PrimitiveComponent|SetLinearDamping (Variables|/Script/Engine.Character|GetCapsuleComponent _playervum_ref) 0.01))

(event EventBeginPlay)

(event Collision|EventActorBeginOverlap
  (params (OtherActor :type Actor%20Object%20Reference)))

(fn ConstructionScript)