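; BP_Laser is a laser beam actor that stretches to whatever blocks it and briefly shrinks the player on contact.
; BeginPlay tints the beam mesh through a dynamic material instance.
; Each tick, a box trace along the up vector scales the mesh to the hit distance or full range, and notifies BPI_Lasers actors when hit or no longer hit, supporting bounces.
; Overlapping a Player-tagged BP_Vum halves its flipbook scale for one second.
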(event OnComponentBeginOverlap(SM_Parent)
  (params (OverlappedComponent :type Primitive%20Component%20Object%20Reference) (OtherActor :type Actor%20Object%20Reference) (OtherComp :type Primitive%20Component%20Object%20Reference) (OtherBodyIndex :type Integer) (bFromSweep :type Boolean) (SweepResult :type Hit%20Result%20Structure%20%28by%20ref%29))
  (bind _asbp_vum (Utilities|Casting|CastToBP_Vum OtherActor))
  (bind _output_get (Variables|Default|SetPlayerRef _asbp_vum))
  (if (Actor|ActorHasTag OtherActor "Player")
    (Transformation|SetWorldScale3D (Variables|/Game/Blueprint/Player_Vum/BP_Vum.BP_Vum_C|GetPaperFlipbook _output_get) "0.500000,0.500000,0.500000")
    (Utilities|FlowControl|Delay 1.0)
    (Transformation|SetWorldScale3D (Variables|/Game/Blueprint/Player_Vum/BP_Vum.BP_Vum_C|GetPaperFlipbook _output_get) "1.000000,1.000000,1.000000")))

(event EventBeginPlay
  (CallFunction|ChangeColor))

(event EventTick
  (params (DeltaSeconds :type Float%20%28single-precision%29))
  (CallFunction|SetEndPoint))

(fn ConstructionScript
  (|CallParentFunction))

(fn ChangeColor
  (bind _returnvalue (Rendering|Material|CreateDynamicMaterialInstance (Variables|Default|GetSM_Parent) 0 "/Game/Blueprint/Assets/LaserBeam/M_Laser.M_Laser" "None" :!class /Script/Engine.PrimitiveComponent))
  (Rendering|Material|SetVectorParameterValue _returnvalue "Color" (Variables|Default|GetLaserColor) :!class /Script/Engine.MaterialInstanceDynamic))

(fn SetEndPoint
  (bind _returnvalue (Transformation|GetActorLocation))
  (bind _returnvalue_2 (Transformation|GetActorUpVector))
  (bind _returnvalue_3 (* _returnvalue_2 2.0))
  (bind _returnvalue_4 (+ _returnvalue _returnvalue_3))
  (bind _outhit (Collision|BoxTraceByChannel _returnvalue_4 (+ _returnvalue_4 (* _returnvalue_2 (Variables|Default|GetLaser%20Range))) "0.500000,0.500000,0.500000" "0, 0, 0" "TraceTypeQuery1" false 0 "None"))
  (bind _output_get (LocalVariables|SetL_Hitinfo _outhit))
  (LocalVariables|SetL_HitActor (.HitActor (Collision|BreakHitResult _output_get)))
  (Transformation|SetWorldScale3D (Variables|Default|GetSM_Parent) (Math|Vector|MakeVector 0.05 0.05 (Math|Float|SelectFloat (/ (+ (.Distance (Collision|BreakHitResult _output_get)) 1.0) 1e+02) (/ (Variables|Default|GetLaser%20Range) 1e+02) (.bBlockingHit (Collision|BreakHitResult _output_get)))))
  (Utilities|FlowControl|Sequence
    (:then_0
      (if (!= (LocalVariables|GetL_HitActor) (Variables|Default|GetLasHitActor))
        (if (Utilities|DoesObjectImplementInterface (Variables|Default|GetLasHitActor) "/Game/Blueprint/Assets/LaserBeam/BPI_Lasers.BPI_Lasers_C")
          (Class|BPILasers|LaserBounce(Message) (Variables|Default|GetLasHitActor) self false (LocalVariables|GetL_Hitinfo))
          (Development|PrintString "Hello"))
        (elif (Utilities|DoesObjectImplementInterface (LocalVariables|GetL_HitActor) "/Game/Blueprint/Assets/LaserBeam/BPI_Lasers.BPI_Lasers_C")
          (Class|BPILasers|LaserBounce(Message) (LocalVariables|GetL_HitActor) self true (LocalVariables|GetL_Hitinfo)))))
    (:then_1
      (bind _l_hitactor (LocalVariables|GetL_HitActor)
        (:then
          (Variables|Default|SetLasHitActor _l_hitactor))
        (:else)))))