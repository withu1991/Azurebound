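; BP_LaserTarget is a laser puzzle target that lights up in the color of the laser hitting it.
; LaserBounce stores the hit response as its active state and passes the laser's color to PuzzleSolved.
; PuzzleSolved creates a dynamic material instance on SMParent at each call, setting Base Color to the laser color when active or dark grey otherwise.
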(event EventBeginPlay)

(fn ConstructionScript
  (|CallParentFunction))

(fn PuzzleSolved
  (params (Color%20Laser :type Linear%20Color%20Structure))
  (bind _returnvalue (Rendering|Material|CreateDynamicMaterialInstance (Variables|Default|GetSM_Parent) 0 0 "None" :!class /Script/Engine.PrimitiveComponent))
  (Rendering|Material|SetVectorParameterValue _returnvalue "Base Color" (Math|Color|SelectColor Color%20Laser "(R=0.235120,G=0.235120,B=0.235120,A=1.000000)" (Variables|Default|GetisActive)) :!class /Script/Engine.MaterialInstanceDynamic))

(fn LaserBounce
  (params (LaserHit :type BP%20Laser%20Object%20Reference) (HitResponse :type Boolean) (HitInformation :type Hit%20Result%20Structure))
  (Variables|Default|SetisActive HitResponse)
  (CallFunction|PuzzleSolved (Variables|/Game/Blueprint/Assets/LaserBeam/BP_LasersParent.BP_LasersParent_C|GetLaserColor LaserHit))
  (return 0))