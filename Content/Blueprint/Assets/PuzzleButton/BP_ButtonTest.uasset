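; BP_ButtonTest is a puzzle floor button that enables puzzle start while pressed.
; Overlap by a Player or Jack-tagged actor sets CanStartPuzzle on the cached BP_Vum, which only the Player branch assigns.
; A Timeline lowers the sprite, reversing on end overlap.
; Its updates trigger a DoOnce that briefly shows the puzzle button text, resetting unless the Vum's IsButtonPressed is set.
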(event OnComponentBeginOverlap(Buttoncollision)
  (params (OverlappedComponent :type Primitive%20Component%20Object%20Reference) (OtherActor :type Actor%20Object%20Reference) (OtherComp :type Primitive%20Component%20Object%20Reference) (OtherBodyIndex :type Integer) (bFromSweep :type Boolean) (SweepResult :type Hit%20Result%20Structure%20%28by%20ref%29))
  (if (Actor|ActorHasTag OtherActor "Player")
    (bind _asbp_vum (Utilities|Casting|CastToBP_Vum OtherActor))
    (bind _output_get (Variables|Default|SetPlayerVum%20Ref _asbp_vum))
    (Variables|/Game/Blueprint/Player_Vum/BP_Vum.BP_Vum_C|SetcanStartPuzzle _output_get true :!label _label)
    (bind _newtrack_0 (Timeline|Timeline Play)
      (:Update
        (Transformation|SetRelativeLocation (Variables|Default|GetPaperSprite) (Math|Vector|MakeVector 0.0 0.0 (Math|Float|Lerp 0.0 -2e+01 _newtrack_0)) false false)
        (Utilities|FlowControl|DoOnce false :!label _label_2
          (:Completed
            (Variables|/Script/UMG.Widget|SetVisibility (Variables|/Game/UI/WB_PickUp.WB_PickUp_C|GetPuzzleButtonText (Variables|/Game/UI/WB_Player.WB_Player_C|GetWB_PickUpRef (Variables|/Game/Blueprint/Player_Vum/BP_Vum.BP_Vum_C|GetWB%20Player%20Ref (Variables|Default|GetPlayerVum%20Ref)))) "Visible")
            (Utilities|FlowControl|Delay 1.0)
            (Variables|/Script/UMG.Widget|SetVisibility (Variables|/Game/UI/WB_PickUp.WB_PickUp_C|GetPuzzleButtonText (Variables|/Game/UI/WB_Player.WB_Player_C|GetWB_PickUpRef (Variables|/Game/Blueprint/Player_Vum/BP_Vum.BP_Vum_C|GetWB%20Player%20Ref (Variables|Default|GetPlayerVum%20Ref)))) "Hidden")
            (if (not (Variables|/Game/Blueprint/Player_Vum/BP_Vum.BP_Vum_C|GetisButtonPressed? (Variables|Default|GetPlayerVum%20Ref)))
              (goto _label_2 Reset))))))
    (elif (Actor|ActorHasTag OtherActor "Jack")
      (goto _label))))

(event OnComponentEndOverlap(Buttoncollision)
  (params (OverlappedComponent :type Primitive%20Component%20Object%20Reference) (OtherActor :type Actor%20Object%20Reference) (OtherComp :type Primitive%20Component%20Object%20Reference) (OtherBodyIndex :type Integer))
  (bind _playervum_ref (Variables|Default|GetPlayerVum%20Ref))
  (Utilities|IsValid _playervum_ref
    (:Is%20Valid
      (Variables|/Game/Blueprint/Player_Vum/BP_Vum.BP_Vum_C|SetcanStartPuzzle _playervum_ref false)
      (bind _newtrack_0 (Timeline|Timeline Reverse)
        (:Update
          (Transformation|SetRelativeLocation (Variables|Default|GetPaperSprite) (Math|Vector|MakeVector 0.0 0.0 (Math|Float|Lerp 0.0 -2e+01 _newtrack_0)) false false)
          (Utilities|FlowControl|DoOnce false :!label _label
            (:Completed
              (Variables|/Script/UMG.Widget|SetVisibility (Variables|/Game/UI/WB_PickUp.WB_PickUp_C|GetPuzzleButtonText (Variables|/Game/UI/WB_Player.WB_Player_C|GetWB_PickUpRef (Variables|/Game/Blueprint/Player_Vum/BP_Vum.BP_Vum_C|GetWB%20Player%20Ref (Variables|Default|GetPlayerVum%20Ref)))) "Visible")
              (Utilities|FlowControl|Delay 1.0)
              (Variables|/Script/UMG.Widget|SetVisibility (Variables|/Game/UI/WB_PickUp.WB_PickUp_C|GetPuzzleButtonText (Variables|/Game/UI/WB_Player.WB_Player_C|GetWB_PickUpRef (Variables|/Game/Blueprint/Player_Vum/BP_Vum.BP_Vum_C|GetWB%20Player%20Ref (Variables|Default|GetPlayerVum%20Ref)))) "Hidden")
              (if (not (Variables|/Game/Blueprint/Player_Vum/BP_Vum.BP_Vum_C|GetisButtonPressed? (Variables|Default|GetPlayerVum%20Ref)))
                (goto _label Reset)))))))))

(event EventBeginPlay)

(event Collision|EventActorBeginOverlap
  (params (OtherActor :type Actor%20Object%20Reference)))

(fn ConstructionScript)