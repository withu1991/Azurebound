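; Level 2 puzzle button, a child Blueprint that configures the level name held on the player reference.
; On actor overlap it runs the parent logic, then clears IsButtonPressed on PlayerVumRef and sets its LevelName to LV_Stairs2.
; BeginPlay and construction only call the parent, and Tick is disabled.
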(event EventBeginPlay
  (|CallParentFunction))

(event Collision|EventActorBeginOverlap
  (params (OtherActor :type Actor%20Object%20Reference))
  (|CallParentFunction OtherActor)
  (Variables|/Game/Blueprint/Player_Vum/BP_Vum.BP_Vum_C|SetisButtonPressed? (Variables|Default|GetPlayerVum%20Ref) false)
  (Variables|/Game/Blueprint/Player_Vum/BP_Vum.BP_Vum_C|SetLevel%20Name (Variables|Default|GetPlayerVum%20Ref) "LV_Stairs2"))

(event EventTick
  (params (DeltaSeconds :type Float%20%28single-precision%29))
  (|CallParentFunction DeltaSeconds) ; This node is disabled and will not be called.\nDrag off pins to build functionality.
)

(fn ConstructionScript
  (|CallParentFunction))