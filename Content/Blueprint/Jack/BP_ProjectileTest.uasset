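; BP_ProjectileTest is a test projectile the player (BP_Vum) shoots, treated as a retrievable "Jack" that places a portal on walls.
; Delayed timers enable Pawn overlap to avoid hitting the shooter, then zero the sphere's velocity.
; Overlaps toggle the player's pickup flag.
; Hitting a "Wall"-tagged actor blocks WorldStatic, matches the player's rotation and, after a delay, moves Portal2 there on a fixed Y.
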(event OnComponentBeginOverlap(SphereCollision)
  (params (OverlappedComponent :type Primitive%20Component%20Object%20Reference) (OtherActor :type Actor%20Object%20Reference) (OtherComp :type Primitive%20Component%20Object%20Reference) (OtherBodyIndex :type Integer) (bFromSweep :type Boolean) (SweepResult :type Hit%20Result%20Structure%20%28by%20ref%29))
  (bind _returnvalue (Transformation|GetActorLocation))
  (if (Actor|ActorHasTag OtherActor "Player")
    (Variables|/Game/Blueprint/Player_Vum/BP_Vum.BP_Vum_C|SetcanPickUpJack (Variables|Default|GetPlayerVumRef) true))
  (if (Actor|ActorHasTag OtherActor "Wall")
    (Collision|SetCollisionResponsetoChannel (Variables|Default|GetSphereCollision) "ECC_WorldStatic" "ECR_Block")
    (Transformation|SetWorldRotation (Variables|Default|GetSphere) (Transformation|GetActorRotation (Variables|Default|GetPlayerVumRef)) false false)
    (Utilities|FlowControl|Delay 2.0)
    (Transformation|SetActorLocation (Variables|/Game/Blueprint/Player_Vum/BP_Vum.BP_Vum_C|GetPortal2%20Ref (Variables|Default|GetPlayerVumRef)) (Math|Vector|MakeVector (.x _returnvalue) -3.0 (+ (.z _returnvalue) 5.0)) false false)))

(event OnComponentEndOverlap(SphereCollision)
  (params (OverlappedComponent :type Primitive%20Component%20Object%20Reference) (OtherActor :type Actor%20Object%20Reference) (OtherComp :type Primitive%20Component%20Object%20Reference) (OtherBodyIndex :type Integer))
  (Variables|/Game/Blueprint/Player_Vum/BP_Vum.BP_Vum_C|SetcanPickUpJack (Variables|Default|GetPlayerVumRef) false)
  (Development|PrintString "Can't Pick Up Jack"))

(event EventBeginPlay
  (bind _returnvalue (Actor|GetActorOfClass "/Game/Blueprint/Player_Vum/BP_Vum.BP_Vum_C"))
  (Variables|Default|SetPlayerVumRef _returnvalue)
  (Utilities|FlowControl|Delay 0.5)
  (Collision|SetCollisionResponsetoChannel (Variables|Default|GetSphereCollision) "ECC_Pawn" "ECR_Overlap") ; this is to make sure it doesn't overlap as soon as player shoots
  (Utilities|FlowControl|Delay 1.0)
  (Physics|SetPhysicsLinearVelocity (Variables|Default|GetSphereCollision) "0, 0, 0" false "None") ; to stop the ball movement. (Delete if not needed)
)

(fn ConstructionScript)