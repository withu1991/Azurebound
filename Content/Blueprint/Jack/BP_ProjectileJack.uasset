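; BP_ProjectileJack is a Jack projectile launched along X in BP_Vum's facing direction.
; Timelines set its velocity and lerp gravity scale toward negative, while BeginPlay also multiplies velocity in tiers from the player's ElapsedSeconds.
; On first overlapping a Wall-tagged actor it stops by destroying its movement component, then moves the player's Portal2 there.
; A Player tag check on overlap enables Jack pickup.
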(event OnComponentBeginOverlap(Sphere)
  (params (OverlappedComponent :type Primitive%20Component%20Object%20Reference) (OtherActor :type Actor%20Object%20Reference) (OtherComp :type Primitive%20Component%20Object%20Reference) (OtherBodyIndex :type Integer) (bFromSweep :type Boolean) (SweepResult :type Hit%20Result%20Structure%20%28by%20ref%29))
  (bind _returnvalue (Transformation|GetActorLocation))
  (if (Actor|ActorHasTag "Player")
    (Variables|/Game/Blueprint/Player_Vum/BP_Vum.BP_Vum_C|SetcanPickUpJack (Variables|Default|GetPlayerVum%20Ref) true)
    (elif (Actor|ActorHasTag OtherActor "Wall")
      (Utilities|FlowControl|DoOnce false
        (:Completed
          (Development|PrintString "Hit")
          (Transformation|SetWorldRotation (Variables|Default|GetPaperSprite) (Transformation|GetActorRotation (Variables|Default|GetPlayerVum%20Ref)) false false)
          (Components|DestroyComponent (Variables|Default|GetProjectileMovement))
          (Collision|SetCollisionResponsetoChannel (Variables|Default|GetSphere) "ECC_Pawn" "ECR_Overlap")
          (Transformation|SetActorLocation (Variables|/Game/Blueprint/Player_Vum/BP_Vum.BP_Vum_C|GetPortal2%20Ref (Variables|Default|GetPlayerVum%20Ref)) (Math|Vector|MakeVector (.x _returnvalue) -3.0 (+ (.z _returnvalue) 5.0)) false false))))))

(event OnComponentEndOverlap(Sphere)
  (params (OverlappedComponent :type Primitive%20Component%20Object%20Reference) (OtherActor :type Actor%20Object%20Reference) (OtherComp :type Primitive%20Component%20Object%20Reference) (OtherBodyIndex :type Integer)))

(event Custom|Projectile%20Velocity
  ;[1 1 1] Initial Velocity/Gravity
  (if (Variables|/Game/Blueprint/Player_Vum/BP_Vum.BP_Vum_C|GetisLookingRight? (Variables|Default|GetPlayerVum%20Ref))
    (bind _newtrack_0 (Timeline|GravityTimeline PlayFromStart)
      (:Update
        (Variables|/Script/Engine.ProjectileMovementComponent|SetProjectileGravityScale (Variables|Default|GetProjectileMovement) (Math|Float|Lerp 1.0 -1e+01 _newtrack_0))
        (Variables|/Script/Engine.MovementComponent|SetVelocity (Variables|Default|GetProjectileMovement) "100.000000,0.000000,0.000000")))
    (else
      (bind _newtrack_0_2 (Timeline|Timeline PlayFromStart)
        (:Update
          (Variables|/Script/Engine.ProjectileMovementComponent|SetProjectileGravityScale (Variables|Default|GetProjectileMovement) (Math|Float|Lerp 1.0 -1e+01 _newtrack_0_2))
          (Variables|/Script/Engine.MovementComponent|SetVelocity (Variables|Default|GetProjectileMovement) "-100.000000,0.000000,0.000000"))))))

(event EventBeginPlay
  (bind _projectilemovement (Variables|Default|GetProjectileMovement))
  (bind _projectilemovement_2 (Variables|Default|GetProjectileMovement))
  (bind _projectilemovement_3 (Variables|Default|GetProjectileMovement))
  ;[1 1 1] Setting velocity
  (bind _returnvalue (Actor|GetActorOfClass "/Game/Blueprint/Player_Vum/BP_Vum.BP_Vum_C"))
  (Variables|Default|SetPlayerVum%20Ref _returnvalue)
  (CallFunction|ProjectileVelocity)
  (Utilities|FlowControl|Sequence
    (:then_0
      (if (<= (Variables|/Game/Blueprint/Player_Vum/BP_Vum.BP_Vum_C|GetElapsed%20Seconds (Variables|Default|GetPlayerVum%20Ref)) 0.0)
        (Variables|/Script/Engine.MovementComponent|SetVelocity _projectilemovement (* (Variables|/Script/Engine.MovementComponent|GetVelocity _projectilemovement) "1.000000,0.000000,0.000000"))))
    (:then_1
      (if (and (> (Variables|/Game/Blueprint/Player_Vum/BP_Vum.BP_Vum_C|GetElapsed%20Seconds (Variables|Default|GetPlayerVum%20Ref)) 1.0) (<= (Variables|/Game/Blueprint/Player_Vum/BP_Vum.BP_Vum_C|GetElapsed%20Seconds (Variables|Default|GetPlayerVum%20Ref)) 2.0))
        (Variables|/Script/Engine.MovementComponent|SetVelocity _projectilemovement_2 (* (Variables|/Script/Engine.MovementComponent|GetVelocity _projectilemovement_2) "2.000000,0.000000,0.000000"))))
    (:then_2
      (if (> (Variables|/Game/Blueprint/Player_Vum/BP_Vum.BP_Vum_C|GetElapsed%20Seconds (Variables|Default|GetPlayerVum%20Ref)) 2.0)
        (Variables|/Script/Engine.MovementComponent|SetVelocity _projectilemovement_3 (* (Variables|/Script/Engine.MovementComponent|GetVelocity _projectilemovement_3) "3.000000,0.000000,0.000000"))))))

(fn ConstructionScript)